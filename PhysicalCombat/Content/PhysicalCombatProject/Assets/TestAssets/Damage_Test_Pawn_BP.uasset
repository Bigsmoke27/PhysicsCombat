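; Test pawn for trying out damage logic by firing physical projectiles with adjustable mass.
; On BeginPlay it adds the Default_MC Enhanced Input context, then moves and looks along the control rotation.
; Attack spawns a Projectile_Test_BP ahead of the pawn, passing a mass multiplier that the mouse wheel adjusts within a clamped range.
; The jump input is repurposed to toggle visibility of the level's Damage_Test_Actor_BP through a FlipFlop.
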(event `self.ReceiveBeginPlay`
  ;[1 1 1] Enable input
  (bind _asplayer_controller_bp (cast `/Game/PhysicalCombatProject/FrameWork/PlayerController_BP` (`self.GetController`)))
  (bind _returnvalue (pcsubsystem `EnhancedInputLocalPlayerSubsystem` _asplayer_controller_bp))
  (`/Engine/EditorBlueprintResources/StandardMacros.IsValid` _returnvalue
    (:`Is Valid`
      (`EnhancedInputSubsystemInterface.AddMappingContext` _returnvalue "/Game/PhysicalCombatProject/Assets/Input/Default_MC.Default_MC" 0 (struct)))
    (:`Is Not Valid`
      (`KismetSystemLibrary.PrintString` "No Input SubSystem"))))

(event `EnhancedInput|/Game/PhysicalCombatProject/Assets/Input/Attack_IA`
  (params (ActionValue :type Boolean) (ElapsedSeconds :type "Float (double-precision)") (TriggeredSeconds :type "Float (double-precision)") (InputAction :type "InputAction Object Reference" :default "/Game/PhysicalCombatProject/Assets/Input/Attack_IA.Attack_IA"))
  (bind _returnvalue (`self.GetControlRotation`))
  (bind _massmultiplier (`self.MassMultiplier`))
  (:`Started`
    ;[1 1 1] TestingDamageLogic
    (`|SpawnActorFromClass` "/Game/PhysicalCombatProject/Assets/TestAssets/Projectile_Test_BP.Projectile_Test_BP_C" (`KismetMathLibrary.MakeTransform` (+ (`self.K2_GetActorLocation`) (* (`KismetMathLibrary.GetForwardVector` _returnvalue) 50.0)) _returnvalue) "Undefined" "MultiplyWithRoot" null (!= _massmultiplier 1) _massmultiplier null)))

(event `EnhancedInput|/Game/PhysicalCombatProject/Assets/Input/Move_IA`
  (params (ActionValue :type "Vector2D Structure") (ElapsedSeconds :type "Float (double-precision)") (TriggeredSeconds :type "Float (double-precision)") (InputAction :type "InputAction Object Reference" :default "/Game/PhysicalCombatProject/Assets/Input/Move_IA.Move_IA"))
  (bind _returnvalue (`self.GetControlRotation`))
  (:`Triggered`
    (`self.AddMovementInput` (`KismetMathLibrary.GetForwardVector` _returnvalue) ActionValue_X)
    (`self.AddMovementInput` (`KismetMathLibrary.GetRightVector` _returnvalue) ActionValue_Y)))

(event `EnhancedInput|/Game/PhysicalCombatProject/Assets/Input/Look_IA`
  (params (ActionValue :type "Vector2D Structure") (ElapsedSeconds :type "Float (double-precision)") (TriggeredSeconds :type "Float (double-precision)") (InputAction :type "InputAction Object Reference" :default "/Game/PhysicalCombatProject/Assets/Input/Look_IA.Look_IA"))
  (:`Triggered`
    (`self.AddControllerYawInput` ActionValue_X)
    (`self.AddControllerPitchInput` (* ActionValue_Y -1.0))))

(event `EnhancedInput|/Game/PhysicalCombatProject/Assets/Input/Jump_IA`
  (params (ActionValue :type Boolean) (ElapsedSeconds :type "Float (double-precision)") (TriggeredSeconds :type "Float (double-precision)") (InputAction :type "InputAction Object Reference" :default "/Game/PhysicalCombatProject/Assets/Input/Jump_IA.Jump_IA"))
  (:`Started`
    (bind _returnvalue (`GameplayStatics.GetActorOfClass` "/Game/PhysicalCombatProject/Assets/TestAssets/Damage_Test_Actor_BP.Damage_Test_Actor_BP_C"))
    (bind _isa (`/Engine/EditorBlueprintResources/StandardMacros.FlipFlop`)
      (:`A`
        _)
      (:`B`
        _))
    (`self.SetActorHiddenInGame` _returnvalue _isa)))

(event `InputAxisKey|MouseWheelAxis`
  (params (AxisValue :type "Float (single-precision)"))
  (set `self.MassMultiplier` (`KismetMathLibrary.Clamp` (`KismetMathLibrary.FTrunc` (+ AxisValue (`self.MassMultiplier`))) 1 100)))

(fn `UserConstructionScript`)