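; BP_AmmoPickup is an interactable ammo pickup that adds its ammo to the character who interacts with it.
; InteractionAction searches the character's BPC_WeaponAmmo components for the first one whose AmmoType matches the pickup's.
; It calls IRProcessAmmoIncrease on that component with AmmoCount and destroys itself, so the pickup stays in the world if no type matches.
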(event `self.Interaction Action`
  (params (Character :type "Character Object Reference"))
  (for _array_element (`self.K2_GetComponentsByClass` Character "/Game/BSP_DABB/Blueprints/Components/BPC_WeaponAmmo.BPC_WeaponAmmo_C")
    (if (`|EnumEquality` (`self.AmmoType`) (`/Game/BSP_DABB/Blueprints/Components/BPC_WeaponAmmo.AmmoType` _array_element))
      (`/Game/BSP_DABB/Blueprints/Components/BPC_WeaponAmmo.IR Process Ammo Increase` _array_element (`self.AmmoCount`))
      (`self.K2_DestroyActor`)
      (break))))

(fn `UserConstructionScript`
  (`parent.UserConstructionScript`))