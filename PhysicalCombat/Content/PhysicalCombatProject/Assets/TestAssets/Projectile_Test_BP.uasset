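; Test projectile actor that launches itself forward and reports its impacts to the damage system of whatever it hits.
; On BeginPlay, its Sphere receives a velocity-change impulse along the actor's forward vector, scaled by LaunchForce.
; On hit, it forwards the collision, with hit components swapped to the victim's perspective, to the other actor's DamageComponent_BP, printing a debug message if none exists.
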(event `self.ReceiveBeginPlay`
  (`PrimitiveComponent.AddImpulse` (`self.Sphere`) (* (`self.GetActorForwardVector`) (`self.LaunchForce`)) "None" true)
  (`PrimitiveComponent.AddImpulse` (`self.Sphere`) (* (`self.GetActorForwardVector`) (`self.LaunchForce`)) "None" true))

(event `self.Sphere.OnComponentHit`
  (params (HitComponent :type "PrimitiveComponent Object Reference") (OtherActor :type "Actor Object Reference") (OtherComp :type "PrimitiveComponent Object Reference") (NormalImpulse :type "Vector Structure") (Hit :type "HitResult Structure (by ref)"))
  (set `self.DamageComp` (`self.GetComponentByClass` OtherActor "/Game/PhysicalCombatProject/Assets/Blueprints/Components/DamageComponent_BP.DamageComponent_BP_C"))
  (bind _damagecomp (`self.DamageComp`)
    (:`then`
      (`/Game/PhysicalCombatProject/Assets/Blueprints/Components/DamageComponent_BP.OnComponentHit_Event` _damagecomp OtherComp OtherActor HitComponent NormalImpulse Hit))
    (:`else`
      (`KismetSystemLibrary.PrintString` "NoDamageComponentFound!"))))

(fn `UserConstructionScript`)