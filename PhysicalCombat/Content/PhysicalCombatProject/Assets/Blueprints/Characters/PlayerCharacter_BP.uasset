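; Player character Blueprint that handles Enhanced Input for looking, moving, jumping and interacting.
; BeginPlay adds the default mapping context through the player controller, and movement follows the forward and right vectors of the full control rotation.
; Interact sphere-traces on Visibility along the camera's forward vector and sends UseMessage to the hit actor.
; The TraceOffset helper starts that trace a spring-arm length ahead of the camera, skipping the camera-to-character gap.
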(event `self.ReceiveBeginPlay`
  (bind _asplayer_controller_bp (cast `/Game/PhysicalCombatProject/FrameWork/PlayerController_BP` (`self.GetController`)))
  (bind _returnvalue (pcsubsystem `EnhancedInputLocalPlayerSubsystem` _asplayer_controller_bp))
  (`/Engine/EditorBlueprintResources/StandardMacros.IsValid` _returnvalue
    (:`Is Valid`
      (`EnhancedInputSubsystemInterface.AddMappingContext` _returnvalue "/Game/PhysicalCombatProject/Assets/Input/Default_MC.Default_MC" 0 (struct)))
    (:`Is Not Valid`
      (`KismetSystemLibrary.PrintString` "No Input SubSystem"))))

(event `EnhancedInput|/Game/PhysicalCombatProject/Assets/Input/Look_IA`
  (params (ActionValue :type "Vector2D Structure") (ElapsedSeconds :type "Float (double-precision)") (TriggeredSeconds :type "Float (double-precision)") (InputAction :type "InputAction Object Reference" :default "/Game/PhysicalCombatProject/Assets/Input/Look_IA.Look_IA"))
  (:`Triggered`
    (`self.AddControllerYawInput` ActionValue_X)
    (`self.AddControllerPitchInput` ActionValue_Y)))

(event `EnhancedInput|/Game/PhysicalCombatProject/Assets/Input/Move_IA`
  (params (ActionValue :type "Vector2D Structure") (ElapsedSeconds :type "Float (double-precision)") (TriggeredSeconds :type "Float (double-precision)") (InputAction :type "InputAction Object Reference" :default "/Game/PhysicalCombatProject/Assets/Input/Move_IA.Move_IA"))
  (:`Triggered`
    (`self.AddMovementInput` (`KismetMathLibrary.GetForwardVector` (`self.GetControlRotation`)) ActionValue_X)
    (`self.AddMovementInput` (`KismetMathLibrary.GetRightVector` (`self.GetControlRotation`)) ActionValue_Y)))

(event `EnhancedInput|/Game/PhysicalCombatProject/Assets/Input/Jump_IA`
  (params (ActionValue :type Boolean) (ElapsedSeconds :type "Float (double-precision)") (TriggeredSeconds :type "Float (double-precision)") (InputAction :type "InputAction Object Reference" :default "/Game/PhysicalCombatProject/Assets/Input/Jump_IA.Jump_IA"))
  (:`Started`
    (`self.Jump`))
  (:`Completed`
    (`self.StopJumping`)))

(event `EnhancedInput|/Game/PhysicalCombatProject/Assets/Input/Interact_IA`
  (params (ActionValue :type Boolean) (ElapsedSeconds :type "Float (double-precision)") (TriggeredSeconds :type "Float (double-precision)") (InputAction :type "InputAction Object Reference" :default "/Game/PhysicalCombatProject/Assets/Input/Interact_IA.Interact_IA"))
  (bind _camera (`self.Camera`))
  (bind (_start _end) (`self.TraceOffset` _camera (`SceneComponent.GetForwardVector` _camera) (`SpringArmComponent.TargetArmLength` (`self.SpringArm`)) 300.0))
  (:`Started`
    (bind _outhit (`KismetSystemLibrary.SphereTraceSingle` _start _end 0.0 "TraceTypeQuery1"))
    (message `/Game/PhysicalCombatProject/Assets/Blueprints/DataAssets/Interaction_BPI.Use` (`.HitActor` (`GameplayStatics.BreakHitResult` _outhit)))))

(event `EnhancedInput|/Game/PhysicalCombatProject/Assets/Input/Attack_IA`
  (params (ActionValue :type Boolean) (ElapsedSeconds :type "Float (double-precision)") (TriggeredSeconds :type "Float (double-precision)") (InputAction :type "InputAction Object Reference" :default "/Game/PhysicalCombatProject/Assets/Input/Attack_IA.Attack_IA")))

(fn `TraceOffset`
  (params (Component :type "SceneComponent Object Reference") (Direction :type "Vector Structure") (StartDistance :type "Float (single-precision)") (EndDistance :type "Float (single-precision)"))
  (returns (Start :type "Vector Structure") (End :type "Vector Structure"))
  (bind _returnvalue (+ (`SceneComponent.K2_GetComponentLocation` (`local.Component`)) (* (`local.Direction`) (`local.StartDistance`))))
  (return _returnvalue (+ _returnvalue (* (`local.Direction`) (`local.EndDistance`)))))

(fn `UserConstructionScript`)