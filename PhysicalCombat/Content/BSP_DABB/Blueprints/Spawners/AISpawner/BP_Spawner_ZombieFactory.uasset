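; Zombie spawner that keeps creating BP_Zombie actors at random spots around itself, running only on the server.
; BeginPlay starts a looping timer at the RespawnTimer interval that calls BSP_SpawnAI, with no limit on spawn count.
; Each spawn takes X and Y from random navigable points within Radius of the spawner mesh and Z from SpawnHight.
; It then calls SpawnDefaultController on the new zombie's Instigator.
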(event `SpawnAIServer`
  ;[0.2705 0.2705 0.2705] Spawn AI with timer
  (`/Engine/EditorBlueprintResources/ActorMacros.Switch Has Authority`
    (:`Authority`
      (`KismetSystemLibrary.K2_SetTimer` null "BSP_SpawnAI" (`self.RespawnTimer`) true))))

(event `self.ReceiveBeginPlay`
  ;[0.2705 0.2705 0.2705] Spawn AI with timer
  (`/Engine/EditorBlueprintResources/ActorMacros.Switch Has Authority`
    (:`Authority`
      (`self.SpawnAIServer`))))

(fn `BSP_SpawnAI`
  ;[0.2705 0.2705 0.2705] Set spawn Location and Spawn AI BP
  (`/Engine/EditorBlueprintResources/ActorMacros.Switch Has Authority`
    (:`Authority`
      (bind _returnvalue (`|SpawnActorFromClass` "/Game/BSP_DABB/Blueprints/Characters/AI/Zombie/BP_Zombie.BP_Zombie_C" (`KismetMathLibrary.MakeTransform` (`KismetMathLibrary.MakeVector` (.x (`NavigationSystemV1.K2_GetRandomLocationInNavigableRadius` (`SceneComponent.K2_GetComponentLocation` (`self.SpwnerMesh`)) (`self.Radius`) null null)) (.y (`NavigationSystemV1.K2_GetRandomLocationInNavigableRadius` (`SceneComponent.K2_GetComponentLocation` (`self.SpwnerMesh`)) (`self.Radius`) null null)) (`self.SpawnHight`))) "AdjustIfPossibleButAlwaysSpawn" "MultiplyWithRoot" null null))
      (`Pawn.SpawnDefaultController` (`Actor.Instigator` _returnvalue)))))

(fn `UserConstructionScript`)