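; Blueprint function library for BSP_DABB that resolves hit bones or damaged-parent enums to body regions and sever points.
; Both functions read DT_HitBoneMappingToDamagedParent and return a DamagedParent with its SeverPoint.
; The bone lookup fetches the row by name, falling back to a Torso sever point.
; The enum lookup scans rows for the first matching parent, returning a None sever point when nothing matches.
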(fn `BSP_GetParentEnumHitParent`
  (params (Hitbone :type "/Game/BSP_DABB/Enumerator/ENUM_BoneParents Enum" :default "NewEnumerator0"))
  (returns (DamagedParent :type "/Game/BSP_DABB/Enumerator/ENUM_BoneParents Enum") (SeverPoint :type Name))
  (bind _outrownames (`DataTableFunctionLibrary.GetDataTableRowNames` "/Game/BSP_DABB/Blueprints/DataTable/DT_HitBoneMappingToDamagedParent.DT_HitBoneMappingToDamagedParent"))
  (for _array_element _outrownames
    (bind _returnvalue (`|GetDataTableRow` "/Game/BSP_DABB/Blueprints/DataTable/DT_HitBoneMappingToDamagedParent.DT_HitBoneMappingToDamagedParent" _array_element)
      (:`then`
        (bind (_damagedparent _severpoint) (break `/Game/BSP_DABB/Structure/FBoneMapping` _returnvalue))
        (if (`|EnumEquality` _damagedparent Hitbone)
          (return _damagedparent _severpoint)))))
  (return "NewEnumerator6" "None"))

(fn `BSP_GetParentFromHitBone`
  (params (Hitbone :type Name))
  (returns (DamagedParent :type "/Game/BSP_DABB/Enumerator/ENUM_BoneParents Enum") (SeverPoint :type Name))
  (bind _returnvalue (`|GetDataTableRow` "/Game/BSP_DABB/Blueprints/DataTable/DT_HitBoneMappingToDamagedParent.DT_HitBoneMappingToDamagedParent" Hitbone)
    (:`then`
      (bind (_damagedparent _severpoint) (break `/Game/BSP_DABB/Structure/FBoneMapping` _returnvalue))
      (return _damagedparent _severpoint))
    (:`RowNotFound`
      (return "NewEnumerator3" "Torso"))))