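; Character interaction component that finds BP_InteractableObject actors under the camera and lets the owning character interact with them.
; For non-AI characters, a looping timer line-traces forward from the third-person camera and sends start/end focus calls as the target changes.
; A DoOnce, re-armed on new focus, triggers a delayed end-focus that clears the last target.
; Interact_Server repeats the trace and calls InteractionAction on the hit object.
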(event `self.Initialise`
  (params (Owning :type "/Game/BSP_DABB/Structure/FBoneBreak_Owning Structure") (ActiveWeapon :type "Actor Object Reference"))
  ;[1 1 1] Initialise Main Values
  (set `self.OwningCharacter` Owning_Character_2_63B5062B4A1FAC8E7F2879AA80A38350)
  (set `self.Owning_Camera` Owning_ThirdPersonCamera_20_9BAAE1F84BFDA624F16C26BA3FBF2833)
  (set `self.bIsAI` Owning_IsCharacterAI_26_54F716A6436236A33A4D6DA56ACA7697)
  (set `self.Owning Spring Arm` Owning_SpringArm_29_69390BC44F54172733B672BA6077AFFB))

(event `self.ReceiveBeginPlay`
  ;[1 1 1] Begin Play
  (`/Engine/EditorBlueprintResources/StandardMacros.IsValid` (`self.OwningCharacter`)
    (:`Is Valid`
      (if (not (`self.bIsAI`))
        (`self.BeginPlay_LocalClient`)))))

(event `BeginPlay_LocalClient`
  ;[1 1 1] Initiate Scan Function
  (if (not (`self.bIsAI`))
    (`KismetSystemLibrary.K2_SetTimer` null "f_Check_Focus" 0.3 true)))

(event `ClientHandleFocus`
  (bind _usableactor (`self.f_Trace_For_Interactior`))
  (`/Engine/EditorBlueprintResources/StandardMacros.IsValid` _usableactor
    (:`Is Valid`
      (bind (_asbp_interactable_object _bsuccess) (cast `/Game/BSP_DABB/Blueprints/Interaction/BP_InteractableObject` _usableactor :!pure true))
      (if _bsuccess
        (`|ExecutionSequence`
          (:`then_0`
            ;[1 1 1] End Focus
            (if (!= (`self.LastUsableActor`) _usableactor)
              (set `self.IsNewFocus` true)
              (if (and (`KismetSystemLibrary.IsValid` (`self.LastUsableActor`)) (!= (`self.LastUsableActor`) _usableactor))
                (`/Game/BSP_DABB/Blueprints/Interaction/BP_InteractableObject.Interaction End Focus` (`self.LastUsableActor`) (`self.OwningCharacter`)))))
          (:`then_1`
            ;[1 1 1] Start Focus
            (set `self.LastUsableActor` _asbp_interactable_object)
            (if (`self.IsNewFocus`)
              (`/Game/BSP_DABB/Blueprints/Interaction/BP_InteractableObject.Interaction Start Focus` (`self.LastUsableActor`) (`self.OwningCharacter`))
              (set `self.IsNewFocus` false)
              (goto _label :!via `Reset`)
              (else
                (`/Engine/EditorBlueprintResources/StandardMacros.DoOnce` false :!label _label
                  (:`Completed`
                    (`KismetSystemLibrary.Delay` 1.0)
                    (`/Game/BSP_DABB/Blueprints/Interaction/BP_InteractableObject.Interaction End Focus` (`self.LastUsableActor`) (`self.OwningCharacter`))
                    (set `self.IsNewFocus` false)
                    (set `self.LastUsableActor` null)))))))))))

(event `Interact_Server`
  (bind _usableactor (`self.f_Trace_For_Interactior`))
  (bind (_asbp_interactable_object _bsuccess) (cast `/Game/BSP_DABB/Blueprints/Interaction/BP_InteractableObject` _usableactor :!pure true))
  ;[1 1 1] Is Object Intractable
  (if _bsuccess
    (`/Game/BSP_DABB/Blueprints/Interaction/BP_InteractableObject.Interaction Action` _asbp_interactable_object (`self.OwningCharacter`))))

(fn `f_Check_Focus`
  (`self.ClientHandleFocus`)
  (return))

(fn `f_Trace_For_Interactior`
  (returns (UsableActor :type "Object Object Reference"))
  (bind _owning_camera (`self.Owning_Camera`))
  (bind _returnvalue (`SceneComponent.K2_GetComponentLocation` _owning_camera))
  (bind _outhit (`KismetSystemLibrary.LineTraceSingle` _returnvalue (+ _returnvalue (* (`SceneComponent.GetForwardVector` _owning_camera) (`self.TraceDistance`))) "TraceTypeQuery1" false (`|MakeArray` (`self.OwningCharacter`) :!type "Actor Object Reference")))
  (return (`.HitActor` (`GameplayStatics.BreakHitResult` _outhit))))

(fn `SetCharacterData`
  (returns (CharacterData :type "/Game/BSP_DABB/Structure/FInteraction_Character_Data Structure"))
  (return))