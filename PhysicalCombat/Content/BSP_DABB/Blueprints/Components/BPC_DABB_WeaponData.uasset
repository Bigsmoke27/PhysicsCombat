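; Weapon data component for BP_Weapon_Master that selects weapon animations matching the owning character's stage of damage.
; It caches the owning character, its bone data component and third-person camera on initialisation.
; It reads the damage stage from bone data, finds the matching entry in the weapon's animation state list, and tells any active weapon to update its offset.
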(event `self.Initialise`
  (params (Owning :type "/Game/BSP_DABB/Structure/FBoneBreak_Owning Structure") (ActiveWeapon :type "Actor Object Reference"))
  ;[0.07451 0.1216 0.2706] Set a reference to the OwningCharacter, BoneData, and the ActiveWeapon (Initialised from the EventBeginPlay of the owning character)
  (set `self.OwningCharacter` Owning_Character_2_63B5062B4A1FAC8E7F2879AA80A38350)
  (set `self.OwningBoneData` Owning_BoneData_15_74E5A5FB48B7165E6FC894B96F1CFEF6)
  (set `self.PlayerCamera` Owning_ThirdPersonCamera_20_9BAAE1F84BFDA624F16C26BA3FBF2833))

(event `/Game/BSP_DABB/Blueprints/Interfaces/BPI_DABB_WeaponData.SetWeaponData`
  (params (BoneDataComponent :type "/Game/BSP_DABB/Blueprints/Components/BPC_DABB_BoneData Object Reference"))
  (set `self.OwningBoneData` BoneDataComponent))

(fn `f_DABB_Get_StateOfDammage_From_OwningBoneData`
  (bind _activeweaponreference (`self.ActiveWeaponReference`))
  (bind _owningbonedata (`self.OwningBoneData`))
  ;[0.07451 0.1216 0.2706] Get animationstate from owning player reference so that the correct Animation state can be applied to the weapon
  (`/Engine/EditorBlueprintResources/StandardMacros.IsValid` (`self.OwningCharacter`)
    (:`Is Valid`
      (`/Engine/EditorBlueprintResources/StandardMacros.IsValid` _owningbonedata
        (:`Is Valid`
          (set `self.StateOfDamageFromBoneData` (`/Game/BSP_DABB/Blueprints/Components/BPC_DABB_BoneData.StageOfDamage` _owningbonedata))
          (`/Engine/EditorBlueprintResources/StandardMacros.IsValid` _activeweaponreference
            (:`Is Valid`
              (`/Game/BSP_DABB/Blueprints/Weapons/BP_Weapon_Master.Event Update Weapon Offset` _activeweaponreference)
              (return))
            (:`Is Not Valid`
              (return))))))
    (:`Is Not Valid`
      (return))))

(fn `f_DABB_Get_Weapon_Animations`
  (returns (ST_Owning_Charater_Weapon_Animation_State :type "/Game/BSP_DABB/Structure/FWeapon_ActionStates Structure"))
  (bind _activeweaponreference (`self.ActiveWeaponReference`))
  (bind _weaponaminationstate (`/Game/BSP_DABB/Blueprints/Weapons/BP_Weapon_Master.WeaponAminationState` (cast `/Game/BSP_DABB/Blueprints/Weapons/BP_Weapon_Master` (`self.GetOwner`) :!pure true)))
  ;[0.07451 0.1216 0.2706] Update list of animations based on the animation state of ownig character
  (`self.f_DABB_Get_StateOfDammage_From_OwningBoneData`)
  (`/Engine/EditorBlueprintResources/StandardMacros.IsValid` _weaponaminationstate
    (:`Is Valid`
      (for _array_element (`/Game/BSP_DABB/Blueprints/DataAssets/PrimaryDataAssets/BP_PDA_Weapon_Animations.ST_Weapon_Animation_State` _weaponaminationstate)
        (`/Engine/EditorBlueprintResources/StandardMacros.IsValid` (`self.OwningBoneData`)
          (:`Is Valid`
            (for _array_element_2 (`.CharacterDamageState_78_4E68CF9A438E0946E1ACE3919A0EA3F5` (break `/Game/BSP_DABB/Structure/FWeapon_ActionStates` _array_element))
              (if (`|EnumEquality` _array_element_2 (`/Game/BSP_DABB/Blueprints/Components/BPC_DABB_BoneData.StageOfDamage` (`self.OwningBoneData`)))
                (set `self.LocalWeaponDataCurentAnimationState` _array_element)
                (`/Engine/EditorBlueprintResources/StandardMacros.IsValid` _activeweaponreference
                  (:`Is Valid`
                    (`/Game/BSP_DABB/Blueprints/Weapons/BP_Weapon_Master.Event Update Weapon Offset` _activeweaponreference)
                    (return _array_element))
                  (:`Is Not Valid`
                    ;[1 1 1] Reset fir Holster
                    (return _array_element)))))))))))

(fn `GetWeaponData`
  (returns (WeaponDataComponent :type "/Game/BSP_DABB/Blueprints/Components/BPC_DABB_WeaponData Object Reference"))
  (return self))