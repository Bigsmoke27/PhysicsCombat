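; Game mode for the dismemberment game that handles dedicated-server session startup and team-based player respawning.
; On BeginPlay, a dedicated server starts a non-LAN session and, on success, opens the Preview level with the listen option.
; Respawning uses the first valid BP_TEAM_PlayerSpawn matching the player's team and marks it used, otherwise keeping the supplied location.
; It then spawns the given character class there and possesses it with the player's controller.
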(event `self.ReceiveBeginPlay`
  (if (`KismetSystemLibrary.IsDedicatedServer`)
    (`CreateSessionCallbackProxy.CreateSession` (`GameplayStatics.GetPlayerController` 0)
      (:`OnSuccess`
        (`GameplayStatics.OpenLevel` "Preview" true "?listen")
        (bind _returnvalue (`GameplayStatics.GetActorOfClass` null))
        (set `self.SpawnLocation` _returnvalue)))))

(event `ResapwnPlayer`
  (params (PlayerController :type "PlayerController Object Reference") (PlayerCharcter :type "Character Class Reference") (RespawnLocation :type "Transform Structure") (PlayerTeam :type "/Game/BSP_DABB/Enumerator/E_TeamList Enum" :default "NewEnumerator0"))
  (bind _outactors (`GameplayStatics.GetAllActorsOfClass` "/Game/BSP_DABB/Blueprints/Spawners/Player/BP_TEAM_PlayerSpawn.BP_TEAM_PlayerSpawn_C"))
  (for _array_element _outactors
    (if (`/Game/BSP_DABB/Blueprints/Spawners/Player/BP_TEAM_PlayerSpawn.PointIsValid` _array_element)
      (if (`|EnumEquality` (`/Game/BSP_DABB/Blueprints/Spawners/Player/BP_TEAM_PlayerSpawn.TEAM` _array_element) PlayerTeam)
        (set `self.RespawnLocation` (`self.GetTransform` _array_element))
        (`/Game/BSP_DABB/Blueprints/Spawners/Player/BP_TEAM_PlayerSpawn.JustBeenUsed` _array_element)
        (break))))
  (bind _returnvalue (`|SpawnActorFromClass` PlayerCharcter (`self.RespawnLocation`) "AdjustIfPossibleButAlwaysSpawn" "SelectDefaultAtRuntime" null null))
  (`/Engine/EditorBlueprintResources/StandardMacros.IsValid` _returnvalue
    (:`Is Valid`
      (`Controller.Possess` PlayerController _returnvalue))))

(fn `UserConstructionScript`)