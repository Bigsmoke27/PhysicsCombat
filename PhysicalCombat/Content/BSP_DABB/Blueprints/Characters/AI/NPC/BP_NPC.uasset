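; BP_NPC is an NPC character Blueprint that records its spawn point, carries a team, and can switch to ragdoll.
; Its construction script copies the Team value into its BPC_Team component.
; On BeginPlay, only the authority stores the actor's transform as SpawnLocation.
; A helper function disables capsule collision and movement, then sets the mesh to the Ragdoll profile with physics simulation.
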(event `self.ReceiveBeginPlay`
  ;[1 1 1] Set Spawn Location
  (`parent.ReceiveBeginPlay`)
  (`/Engine/EditorBlueprintResources/ActorMacros.Switch Has Authority`
    (:`Authority`
      (set `self.SpawnLocation` (`self.GetTransform`)))))

(fn `BSP_DisableMovementAndRagdoll`
  (bind _mesh (`self.Mesh`))
  (`PrimitiveComponent.SetCollisionEnabled` (`self.CapsuleComponent`) "NoCollision")
  (`CharacterMovementComponent.DisableMovement` (`self.CharacterMovement`))
  (`PrimitiveComponent.SetCollisionProfileName` _mesh "Ragdoll" true)
  (`PrimitiveComponent.SetSimulatePhysics` _mesh true)
  (`PrimitiveComponent.SetCollisionEnabled` (`self.CapsuleComponent`) "NoCollision")
  (return))

(fn `UserConstructionScript`
  (`parent.UserConstructionScript`)
  (set `/Game/BSP_DABB/Blueprints/Components/BPC_Team.BSP_Team` (`self.Team`) (`self.GetComponentByClass` "/Game/BSP_DABB/Blueprints/Components/BPC_Team.BPC_Team_C")))