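; Zombie AI character that integrates the DABB bone-damage component, with example melee attack and death logic.
; BeginPlay retries component initialisation until valid, then passes cached animation data to the AnimBP.
; Point and radial damage feed bone names into DABB, destroying the actor after death.
; AttackBox overlaps with other teams open timed hand-collision windows; only right-hand overlaps deal damage, converting body index to bone name.
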(event `self.ReceiveBeginPlay`
  ;[1 1 1] Set Spawn Location
  (`parent.ReceiveBeginPlay`)
  (set `self.SpawnLocation` (`self.GetTransform`))
  ;[0.07451 0.1216 0.2706] Required for Integration
  ;;[0 0 0] Initialise Components
  (`/Engine/EditorBlueprintResources/StandardMacros.IsValid` (`/Game/BSP_DABB/Blueprints/Components/BPC_DABB_BoneData.Owning_Character_Referance` (`self.BPC_DABB_BoneData`)) :!label _label
    (:`Is Valid`
      (`self.f_DABB_SendComponentAndVariablesToAnimInstance`)
      ;[0.2706 0.227 0.01255] Example Logic only
      (`PrimitiveComponent.IgnoreActorWhenMoving` (`self.AttackBox`) self true)
      (`PrimitiveComponent.IgnoreActorWhenMoving` (`self.AttackHandR`) self true)
      (`PrimitiveComponent.IgnoreActorWhenMoving` (`self.AttackHandL`) self true)
      ;[0.07451 0.1216 0.2706] Required for Integration
      ;;[0 0 0] Set Default Speed top be used by Bone Component
      (`/Engine/EditorBlueprintResources/ActorMacros.Switch Has Authority`
        (:`Authority`
          (`/Game/BSP_DABB/Blueprints/Components/BPC_DABB_BoneData.DABB_SwitchWalkRun_Client` (`self.BPC_DABB_BoneData`) false false))))
    (:`Is Not Valid`
      (`self.f_DABB_InitaliseComponents`)
      (`KismetSystemLibrary.Delay` 0.2)
      (goto _label))))

(event `self.ReceivePointDamage`
  (params (Damage :type "Float (single-precision)") (DamageType :type "DamageType Object Reference") (HitLocation :type "Vector Structure") (HitNormal :type "Vector Structure") (HitComponent :type "PrimitiveComponent Object Reference") (BoneName :type Name) (ShotFromDirection :type "Vector Structure") (InstigatedBy :type "Controller Object Reference") (DamageCauser :type "Actor Object Reference") (HitInfo :type "HitResult Structure (by ref)"))
  (bind _bdead (`/Game/BSP_DABB/Blueprints/Components/BPC_Stats_IsDead.bDead` (`self.BPC_Stats_IsDead`)))
  ;[0.2705 0.2705 0.2705] Damage handling
  ;;[1 1 1] Receive Damage Point
  ;;;[0.07451 0.1216 0.2706] Required for Integration
  (`/Game/BSP_DABB/Blueprints/Components/BPC_DABB_BoneData.DABB_DamageManagment` (`self.BPC_DABB_BoneData`) BoneName Damage)
  ;;[0.2706 0.227 0.01255] Example Logic only
  (if _bdead
    (set `/Game/BSP_DABB/Blueprints/Components/BPC_Team.IsDead` _bdead (`self.BPC_Team`))
    (`KismetSystemLibrary.Delay` 3.0)
    (`self.K2_DestroyActor`)))

(event `self.ReceiveRadialDamage`
  (params (DamageReceived :type "Float (single-precision)") (DamageType :type "DamageType Object Reference") (Origin :type "Vector Structure") (HitInfo :type "HitResult Structure (by ref)") (InstigatedBy :type "Controller Object Reference") (DamageCauser :type "Actor Object Reference"))
  (bind _bdead (`/Game/BSP_DABB/Blueprints/Components/BPC_Stats_IsDead.bDead` (`self.BPC_Stats_IsDead`)))
  ;[0.2705 0.2705 0.2705] Damage handling
  ;;[1 1 1] Receive damage Radial
  ;;;[0.07451 0.1216 0.2706] Required for Integration
  (`/Game/BSP_DABB/Blueprints/Components/BPC_DABB_BoneData.DABB_DamageManagment` (`self.BPC_DABB_BoneData`) (`.HitBoneName` (`GameplayStatics.BreakHitResult` HitInfo)) DamageReceived)
  ;;[0.2706 0.227 0.01255] Example Logic only
  (if _bdead
    (set `/Game/BSP_DABB/Blueprints/Components/BPC_Team.IsDead` _bdead (`self.BPC_Team`))
    (`KismetSystemLibrary.Delay` 3.0)
    (`self.K2_DestroyActor`)))

(event `self.AttackBox.OnComponentBeginOverlap`
  (params (OverlappedComponent :type "PrimitiveComponent Object Reference") (OtherActor :type "Actor Object Reference") (OtherComp :type "PrimitiveComponent Object Reference") (OtherBodyIndex :type Integer) (bFromSweep :type Boolean) (SweepResult :type "HitResult Structure (by ref)"))
  ;[0.2705 0.2705 0.2705] Hand Collision
  ;;[0.07451 0.1216 0.2706] Set Attacking Mode if collision if hit sphere overlaps to play animation
  (if (!= OtherActor self)
    (bind _aitarget (`self.AI_CastToOverlappingComponent` OtherActor))
    (if _aitarget
      (set `self.Attacking` true)
      (`KismetSystemLibrary.Delay` 0.8)
      (`PrimitiveComponent.SetCollisionEnabled` (`self.AttackHandR`) "QueryAndPhysics")
      (`PrimitiveComponent.SetCollisionEnabled` (`self.AttackHandL`) "QueryAndPhysics")
      (`KismetSystemLibrary.Delay` 2.3)
      (set `self.Attacking` false)
      (`PrimitiveComponent.SetCollisionEnabled` (`self.AttackHandR`) "NoCollision")
      (`PrimitiveComponent.SetCollisionEnabled` (`self.AttackHandL`) "NoCollision"))))

(event `self.AttackBox.OnComponentEndOverlap`
  (params (OverlappedComponent :type "PrimitiveComponent Object Reference") (OtherActor :type "Actor Object Reference") (OtherComp :type "PrimitiveComponent Object Reference") (OtherBodyIndex :type Integer))
  ;[0.2705 0.2705 0.2705] Hand Collision
  ;;[0.07451 0.1216 0.2706] Set Attacking Mode if collision if hit sphere overlaps to play animation
  (if (!= OtherActor self)
    (bind _aitarget (`self.AI_CastToOverlappingComponent` OtherActor))
    (if _aitarget
      (`PrimitiveComponent.SetCollisionEnabled` (`self.AttackHandR`) "NoCollision")
      (`PrimitiveComponent.SetCollisionEnabled` (`self.AttackHandL`) "NoCollision"))))

(event `self.AttackHandR.OnComponentBeginOverlap`
  (params (OverlappedComponent :type "PrimitiveComponent Object Reference") (OtherActor :type "Actor Object Reference") (OtherComp :type "PrimitiveComponent Object Reference") (OtherBodyIndex :type Integer) (bFromSweep :type Boolean) (SweepResult :type "HitResult Structure (by ref)"))
  (bind (_bblockinghit _binitialoverlap _time _distance _location _impactpoint _normal _impactnormal _physmat _hitactor _hitcomponent _hitbonename _bonename _hititem _elementindex _faceindex _tracestart _traceend) (`GameplayStatics.BreakHitResult` SweepResult))
  ;[0.2705 0.2705 0.2705] Hand Collision
  (bind (_asskinned_mesh_component _returnvalue) (`self.m_ConvertOverlapColisionToBoneHit` OtherActor OtherComp OtherBodyIndex)
    (:`true`
      (bind _aitarget (`self.AI_CastToOverlappingComponent` OtherActor))
      (if _aitarget
        (`/Engine/EditorBlueprintResources/StandardMacros.IsValid` _hitactor
          (:`Is Valid`
            (`GameplayStatics.ApplyPointDamage` _hitactor 60.0 _normal (`GameplayStatics.MakeHitResult` _bblockinghit _binitialoverlap _time _distance _location _impactpoint _normal _impactnormal _physmat OtherActor _asskinned_mesh_component _returnvalue "None" _hititem 0 _faceindex _tracestart _traceend) null self)))))))

(event `self.ReceiveTick`
  (params (DeltaSeconds :type "Float (single-precision)")))

(fn `AI_CastToOverlappingComponent`
  (params (NewParam :type "Actor Object Reference"))
  (returns (AITarget :type Boolean))
  (bind _returnvalue (`self.GetComponentByClass` NewParam "/Game/BSP_DABB/Blueprints/Components/BPC_Team.BPC_Team_C"))
  (`/Engine/EditorBlueprintResources/StandardMacros.IsValid` NewParam
    (:`Is Valid`
      (`/Engine/EditorBlueprintResources/StandardMacros.IsValid` _returnvalue
        (:`Is Valid`
          (return (`|EnumInequality` (`/Game/BSP_DABB/Blueprints/Components/BPC_Team.BSP_Team` _returnvalue) (`self.Team`))))
        (:`Is Not Valid`
          (return false))))
    (:`Is Not Valid`
      (return false))))

(fn `f_DABB_InitaliseComponents`
  ;[0.01758 0.04711 0.1406] Required for Integration
  (`/Game/BSP_DABB/Blueprints/Components/BPC_DABB_MasterDismember.Initialise` (`self.BPC_DABB_BoneData`) (make `/Game/BSP_DABB/Structure/FBoneBreak_Owning` self null (`self.Mesh`) (`self.CapsuleComponent`) (`self.BPC_DABB_BoneData`) null null (`self.CharacterMovement`) (`self.IsAI`)) null)
  (return))

(fn `f_DABB_SendComponentAndVariablesToAnimInstance`
  (bind _bpc_dabb_bonedata (`self.BPC_DABB_BoneData`))
  (bind _returnvalue (`SkeletalMeshComponent.GetAnimInstance` (`self.Mesh`)))
  ;[1 1 1] Added by Josh
  ;;[1 1 1] Pass the component's variables to the animation blueprint that is listening for it
  (message `/Game/BSP_DABB/Blueprints/Interfaces/BPI_DABB_AnimInstance.SetCharacterAnimations` _returnvalue (make `/Game/BSP_DABB/Structure/FAnimation_BaseMovement` (`/Game/BSP_DABB/Blueprints/Components/BPC_DABB_BoneData.StageOfDamage` _bpc_dabb_bonedata) (`/Game/BSP_DABB/Blueprints/Components/BPC_DABB_BoneData.Cached_Walk_Run` _bpc_dabb_bonedata) (`/Game/BSP_DABB/Blueprints/Components/BPC_DABB_BoneData.Cached_Idle` _bpc_dabb_bonedata) (`/Game/BSP_DABB/Blueprints/Components/BPC_DABB_BoneData.Cached_Attack` _bpc_dabb_bonedata) (`/Game/BSP_DABB/Blueprints/Components/BPC_DABB_BoneData.Cached_RagdollRecoverFromFront` _bpc_dabb_bonedata) (`/Game/BSP_DABB/Blueprints/Components/BPC_DABB_BoneData.Cached_RagdollRecoverFromBack` _bpc_dabb_bonedata)) (`/Game/BSP_DABB/Blueprints/Components/BPC_DABB_BoneData.Cached_AimOffset` _bpc_dabb_bonedata))
  ;;[1 1 1] Pass the owner's component to the anim instance
  (message `/Game/BSP_DABB/Blueprints/Interfaces/BPI_DABB_AnimInstance.SetCharacterComponent` _returnvalue (`self.BPC_DABB_BoneData`)))

(fn `UserConstructionScript`
  (`parent.UserConstructionScript`)
  ;[1 1 1] Set Rotation Speed
  (set `CharacterMovementComponent.RotationRate` (`KismetMathLibrary.MakeRotator` 0.0 0.0 (`self.TurnSpeed`)) (`self.CharacterMovement`)))