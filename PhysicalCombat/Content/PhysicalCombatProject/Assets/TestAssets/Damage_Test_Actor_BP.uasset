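; Test actor for locational damage: a modular skeletal-mesh body whose parts detach when hit.
; The construction script makes each part follow Main's pose and maps bone names to parts, while BeginPlay runs physical animation on Main.
; Damage component reports look up the hit bone's part, clear its leader pose and, after a short delay, simulate its physics.
; Losing a leg or thigh sets Crawling and switches Main to Sleeping_Idle.
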(event `self.ReceiveBeginPlay`
  (bind _physicalanimation (`self.PhysicalAnimation`))
  (bind _body_name (`self.Body Name`))
  (`PhysicalAnimationComponent.SetSkeletalMeshComponent` _physicalanimation (`self.Main`))
  (`PhysicalAnimationComponent.ApplyPhysicalAnimationSettingsBelow` _physicalanimation _body_name (make `PhysicalAnimationData` true 1500.0 100.0 1500.0 100.0) false)
  (`SkeletalMeshComponent.SetAllBodiesBelowSimulatePhysics` (`self.Main`) _body_name true false)
  ;[1 1 1] Receive info about hit
  (add `/Game/PhysicalCombatProject/Assets/Blueprints/Components/DamageComponent_BP.ReportDamage` (`self.DamageComponent_BP`) (`|CreateDelegate` :!event `ReceivedDamageReport`)))

(event `ReceivedDamageReport`
  (params (HitData :type "HitResult Structure"))
  (bind _value (`BlueprintMapLibrary.Map_Find` (`self.BodyMap`) (`SkinnedMeshComponent.GetSocketBoneName` (`self.Main`) HitData_HitBoneName)))
  ;[1 1 1] Receive info about hit
  (`KismetSystemLibrary.PrintString` (`KismetSystemLibrary.GetDisplayName` _value))
  (if (and (!= _value (`self.Main`)) (not (`SceneComponent.IsSimulatingPhysics` _value "None")))
    (`self.Detach Component` _value)))

(event `Detach Component`
  (params (`SK Component` :type "SkeletalMeshComponent Object Reference"))
  (`SkinnedMeshComponent.SetLeaderPoseComponent` `SK Component` null false false)
  (`KismetSystemLibrary.Delay` 0.1)
  (`PrimitiveComponent.SetSimulatePhysics` `SK Component` true)
  (if (or (== `SK Component` (`self.LeftLeg`)) (== `SK Component` (`self.RightLeg`)) (== `SK Component` (`self.RightThigh`)) (== `SK Component` (`self.LeftThigh`)))
    (set `self.Crawling` true)
    (`SkeletalMeshComponent.SetAnimation` (`self.Main`) "/Game/PhysicalCombatProject/Assets/Animations/UE5_DamageAct/Sleeping_Idle.Sleeping_Idle")))

(fn `Physics Sim`
  (params (self2 :type "SkeletalMeshComponent Object Reference") (InSkeletalMeshComponent :type "SkeletalMeshComponent Object Reference"))
  (bind _physicalanimation (`self.PhysicalAnimation`))
  (bind _body_name (`self.Body Name`))
  (`PhysicalAnimationComponent.SetSkeletalMeshComponent` _physicalanimation InSkeletalMeshComponent)
  (`PhysicalAnimationComponent.ApplyPhysicalAnimationSettingsBelow` _physicalanimation _body_name (make `PhysicalAnimationData` true 1000.0 100.0 1000.0 100.0) false)
  (`SkeletalMeshComponent.SetAllBodiesBelowSimulatePhysics` self2 _body_name true false))

(fn `UserConstructionScript`
  (bind _torso (`self.Torso`))
  (bind _rightthigh (`self.RightThigh`))
  (bind _leftleg (`self.LeftLeg`))
  (bind _head (`self.Head`))
  (`SkinnedMeshComponent.SetLeaderPoseComponent` (`self.RightElbow`) (`self.Main`) false false)
  (`SkinnedMeshComponent.SetLeaderPoseComponent` (`self.LeftElbow`) (`self.Main`) false false)
  (`SkinnedMeshComponent.SetLeaderPoseComponent` (`self.LeftShoulder`) (`self.Main`) false false)
  (`SkinnedMeshComponent.SetLeaderPoseComponent` (`self.RightLeg`) (`self.Main`) false false)
  (`SkinnedMeshComponent.SetLeaderPoseComponent` (`self.RightThigh`) (`self.Main`) false false)
  (`SkinnedMeshComponent.SetLeaderPoseComponent` (`self.LeftLeg`) (`self.Main`) false false)
  (`SkinnedMeshComponent.SetLeaderPoseComponent` (`self.LeftThigh`) (`self.Main`) false false)
  (`SkinnedMeshComponent.SetLeaderPoseComponent` (`self.Head`) (`self.Main`) false false)
  (`SkinnedMeshComponent.SetLeaderPoseComponent` (`self.LeftHand`) (`self.Main`) false false)
  (`SkinnedMeshComponent.SetLeaderPoseComponent` (`self.RightHand`) (`self.Main`) false false)
  (`SkinnedMeshComponent.SetLeaderPoseComponent` (`self.RightArm`) (`self.Main`) false false)
  (`SkinnedMeshComponent.SetLeaderPoseComponent` (`self.LeftArm`) (`self.Main`) false false)
  (`SkinnedMeshComponent.SetLeaderPoseComponent` (`self.RightShoulder`) (`self.Main`) false false)
  (`SkinnedMeshComponent.SetLeaderPoseComponent` (`self.Torso`) (`self.Main`) false false)
  (set `self.BodyMap` (`|MakeMap` "head" _head "neck_01" _head "neck_02" _head "None" _torso "pelvis" _torso "spine_01" _torso "spine_02" _torso "spine_03" _torso "spine_04" _torso "spine_05" _torso "clavicle_l" (`self.LeftShoulder`) "clavicle_r" (`self.RightShoulder`) "upperarm_l" (`self.LeftElbow`) "lowerarm_l" (`self.LeftArm`) "hand_l" (`self.LeftHand`) "upperarm_r" (`self.RightElbow`) "lowerarm_r" (`self.RightArm`) "hand_r" (`self.RightHand`) "thigh_l" (`self.LeftThigh`) "calf_l" _leftleg "foot_l" _leftleg "thigh_r" _rightthigh "calf_r" _rightthigh "foot_r" (`self.RightLeg`) :!type "Name")))