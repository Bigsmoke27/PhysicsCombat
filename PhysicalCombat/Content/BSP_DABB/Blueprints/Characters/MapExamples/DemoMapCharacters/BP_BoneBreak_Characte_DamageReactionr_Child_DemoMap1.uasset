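; Demo-map child of the bone-break damage-reaction character that arms itself with a rifle shortly after play begins.
; After a delay it spawns a BP_Rifle, stores it as the weapon container's primary and attaches it to a holster socket.
; After a second delay it switches to that rifle, using the server call only with authority, then updates bone data and plays swap animations.
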(event `self.ReceiveBeginPlay`
  ;[1 1 1] Add Weapon To Example macp character
  (`parent.ReceiveBeginPlay`)
  (`KismetSystemLibrary.Delay` 5.0)
  (bind _returnvalue (`|SpawnActorFromClass` "/Game/BSP_DABB/Blueprints/Weapons/BP_Rifle.BP_Rifle_C" (`self.GetTransform` self) "AlwaysSpawn" "OverrideRootScale" self self))
  (set `/Game/BSP_DABB/Blueprints/Weapons/BP_Weapon_Master.bIsInuse` true _returnvalue)
  (set `/Game/BSP_DABB/Blueprints/Weapons/BP_Weapon_Master.bIsAtatched` true _returnvalue)
  (bind _output_get (set `/Game/BSP_DABB/Blueprints/Components/BPC_Weapon_Container.Weapon_Primary` _returnvalue (`self.BPC_Weapon_Container`)))
  (`self.K2_AttachToActor` _output_get self "Holster_Secondary" "SnapToTarget" "SnapToTarget" "SnapToTarget" false)
  (`KismetSystemLibrary.Delay` 5.0)
  (`/Engine/EditorBlueprintResources/StandardMacros.IsValid` _output_get
    (:`Is Valid`
      (`/Engine/EditorBlueprintResources/ActorMacros.Switch Has Authority`
        (:`Authority`
          (`self.DABB_Switch_Weapon_Server` _output_get))
        (:`Remote`
          _))
      (`/Game/BSP_DABB/Blueprints/Components/BPC_DABB_BoneData.f_DABB_Switch_Weapons` (`self.BPC_DABB_BoneData`) _output_get)
      (`self.DABB_PlayWeaponSwapAnimations`))))

(fn `UserConstructionScript`
  (`parent.UserConstructionScript`))